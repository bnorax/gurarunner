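; BP_PowerUpBase is the base actor for collectible power-ups in an endless runner shooter.
; It binds to its parent tile's destroyed event on BeginPlay, so it is removed along with that tile.
; When the player pawn overlaps its mesh, it fires OnCollected with that pawn, which here only plays a sound and destroys the power-up.
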(event OnComponentBeginOverlap(PowerUpMesh)
  (params (OverlappedComponent :type Primitive%20Component%20Object%20Reference) (OtherActor :type Actor%20Object%20Reference) (OtherComp :type Primitive%20Component%20Object%20Reference) (OtherBodyIndex :type Integer) (bFromSweep :type Boolean) (SweepResult :type Hit%20Result%20Structure%20%28by%20ref%29))
  ;[1 1 1] Detect player overlap and destroy the PowerUp when collected
  (bind _asbp_endless_runner_shooter_pawn_base (Utilities|Casting|CastToBP_EndlessRunnerShooterPawnBase OtherActor))
  (CallFunction|OnCollected _asbp_endless_runner_shooter_pawn_base))

(event Custom|OnParentTileDestroyed
  (params (DestroyedActor :type Actor%20Object%20Reference))
  ;[1 1 1] Destroy when parent tile is destroyed
  (Actor|DestroyActor))

(event Custom|OnCollected
  (params (endlessRunnerShooterPawnBase :type BP%20Endless%20Runner%20Shooter%20Pawn%20Base%20Object%20Reference))
  ;[1 1 1] Detect player overlap and destroy the PowerUp when collected
  (Audio|PlaySoundatLocation "/Game/EndlessRunnerShooterTemplate/Sounds/Wavs/GuraA.GuraA" "0, 0, 0" "0, 0, 0" 0.5 1.0 0.0 0 0 0)
  (Actor|DestroyActor))

(event EventBeginPlay
  (bind _parenttile (Variables|Default|GetparentTile))
  ;[1 1 1] Destroy when parent tile is destroyed
  (Utilities|IsValid _parenttile
    (:Is%20Valid
      (Game|AssignOnDestroyed _parenttile (delegate Custom|OnParentTileDestroyed)))))

(fn ConstructionScript)